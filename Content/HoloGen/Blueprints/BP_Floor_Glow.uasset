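; BP_Floor_Glow is a configurable HoloGen actor that renders a glowing floor particle effect through a Niagara component.
; All setup runs in the Construction Script, with no runtime event logic.
; It builds a dynamic instance of MM_FloorGlow_Particles with opacity, emissive strength and a mask texture.
; That material is passed to Niagara along with box size, spawn rate, particle size range and two colors.
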(fn `UserConstructionScript`
  (`|ExecutionSequence`
    (:`then_0`
      (bind _returnvalue (`KismetMaterialLibrary.CreateDynamicMaterialInstance` "/Game/HoloGen/Materials/Master/MM_FloorGlow_Particles.MM_FloorGlow_Particles"))
      (set `self.DynamicMat_FloorGlow` _returnvalue)
      (`MaterialInstanceDynamic.SetScalarParameterValue` (`self.DynamicMat_FloorGlow`) "Opacity Master" (`self.Opacity`))
      (`MaterialInstanceDynamic.SetScalarParameterValue` (`self.DynamicMat_FloorGlow`) "EmissivePower" (`self.Emissive Strength`))
      (`MaterialInstanceDynamic.SetTextureParameterValue` (`self.DynamicMat_FloorGlow`) "Glow_Mask" (`self.Mask Texture`)))
    (:`then_1`
      (`NiagaraComponent.SetVariableMaterial` (`self.Niagara`) "Source_Material" (`self.DynamicMat_FloorGlow`))
      (`NiagaraComponent.SetVariableVec3` (`self.Niagara`) "BoxSize" (`self.Box Size`))
      (`NiagaraComponent.SetVariableFloat` (`self.Niagara`) "SpawnRate" (`self.SpawnRate`))
      (`NiagaraComponent.SetVariableFloat` (`self.Niagara`) "Particle_Size_Min" (`self.Size Min`))
      (`NiagaraComponent.SetVariableFloat` (`self.Niagara`) "Particle_Size_Max" (`self.Size Max`))
      (`NiagaraComponent.SetVariableLinearColor` (`self.Niagara`) "Color1" (`self.Color 1`))
      (`NiagaraComponent.SetVariableLinearColor` (`self.Niagara`) "Color2" (`self.Color 2`)))))