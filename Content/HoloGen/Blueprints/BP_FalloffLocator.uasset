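; BP_FalloffLocator is a placeable locator that defines a falloff distance for the BP_HoloGen actors in a level.
; Its construction script locks world scale to one, clamps FallOffDistance to a small positive minimum and sizes the sphere component to 80% of that distance.
; It then calls FalloffUpdate on every BP_HoloGen, so they refresh whenever the locator is reconstructed.
; It has no active runtime logic.
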(fn `UserConstructionScript`
  (`SceneComponent.SetWorldScale3D` (`self.DefaultSceneRoot`) (1.0 1.0 1.0))
  (if (<= (`self.FallOff_Distance`) 0.001)
    (set `self.FallOff_Distance` 0.001))
  (`SphereComponent.SetSphereRadius` (`self.Sphere`) (* (`self.FallOff_Distance`) 0.8) false)
  (bind _outactors (`GameplayStatics.GetAllActorsOfClass` "/Game/HoloGen/Blueprints/BP_HoloGen.BP_HoloGen_C"))
  (for _array_element _outactors
    (`/Game/HoloGen/Blueprints/BP_HoloGen.FalloffUpdate` _array_element)))