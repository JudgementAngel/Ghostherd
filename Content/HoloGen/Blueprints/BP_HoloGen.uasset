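; BP_HoloGen is a configurable hologram generator that renders a static or skeletal mesh with a masked texture effect plus Niagara pixel and string particles.
; The construction script picks the Niagara system and creates dynamic materials, feeding them exposed settings for style, color, noise, scanlines and glitching.
; With falloff tools enabled, Tick pushes the FalloffLocator's position and distance to particles and mesh material to animate the effect.
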(event `self.ReceiveTick`
  (params (DeltaSeconds :type "Float (single-precision)"))
  (if (`self.Activate Falloff Tools?`)
    (`self.FalloffUpdate`)))

(fn `FalloffUpdate`
  (bind _returnvalue (`self.K2_GetActorLocation` self))
  (bind _returnvalue_2 (`self.K2_GetActorLocation` (`self.Falloff Locator`)))
  (bind _falloff_distance (`/Game/HoloGen/Blueprints/BP_FalloffLocator.FallOff_Distance` (`self.Falloff Locator`)))
  (if (`self.Activate Falloff Tools?`)
    (`|ExecutionSequence`
      (:`then_0`
        ;[1 1 1] Update falloff params to niagara system when anim tools are on
        (`NiagaraComponent.SetVariableFloat` (`self.Niagara`) "Falloff_FalloffSize" _falloff_distance)
        (`MaterialInstanceDynamic.SetScalarParameterValue` (`self.DynamicMeshMat`) "Mat_FalloffSize" _falloff_distance)
        (`NiagaraComponent.SetVariableVec3` (`self.Niagara`) "FalloffLocation" _returnvalue_2)
        (`MaterialInstanceDynamic.SetVectorParameterValue` (`self.DynamicMeshMat`) "Mat_FalloffLocation" (`KismetMathLibrary.Conv_VectorToLinearColor` _returnvalue_2))
        (`NiagaraComponent.SetVariableFloat` (`self.Niagara`) "Scale In Height" (`self.Scale-in Height`)))
      (:`then_1`
        (`MaterialInstanceDynamic.SetScalarParameterValue` (`self.DynamicMeshMat`) "Pulse Intensity" (`self.Edge Emissive Intensity`))
        (`MaterialInstanceDynamic.SetScalarParameterValue` (`self.DynamicMeshMat`) "Falloff Edge Scale" (`self.Edge Detail Scale`))))
    (else
      ;[1 1 1] Keep Falloff at actor location when anim tools are off
      (`NiagaraComponent.SetVariableVec3` (`self.Niagara`) "FalloffLocation" _returnvalue)
      (`MaterialInstanceDynamic.SetVectorParameterValue` (`self.DynamicMeshMat`) "Mat_FalloffLocation" (`KismetMathLibrary.Conv_VectorToLinearColor` _returnvalue)))))

(fn `PixelTypeSwitchbox`
  (params (`2D Vector In` :type "Float (double-precision)"))
  (returns (`2D Vector Out` :type "Float (double-precision)"))
  (return (select `/Game/HoloGen/Blueprints/Core/Enum_ParticleType` (`self.Pixel Type`) :`NewEnumerator0` `2D Vector In` :`NewEnumerator1` (* `2D Vector In` 5.0) :`NewEnumerator2` (* `2D Vector In` 1.5) :`NewEnumerator3` `2D Vector In`)))

(fn `UserConstructionScript`
  (bind _mesh (`self.Mesh`))
  (bind _skmesh (`self.SKMesh`))
  (bind (_bchannel0 _bchannel1 _bchannel2) (break `LightingChannels` (`self.Lighting Channel`)))
  (`NiagaraComponent.SetAsset` (`self.Niagara`) (select `bool` (`self.Use Skeletal Mesh?`) :`false` "/Game/HoloGen/Particles/Nsystem_MeshParticles_Constant_BP.Nsystem_MeshParticles_Constant_BP" :`true` "/Game/HoloGen/Particles/Nsystem_SKMeshParticles_Constant_BP.Nsystem_SKMeshParticles_Constant_BP" :!type "NiagaraSystem Object Reference") false)
  (`|ExecutionSequence`
    (:`then_0`
      ;[1 1 1] Mesh Setup
      (`SceneComponent.SetVisibility` (`self.SKMesh`) (`self.Use Skeletal Mesh?`) false)
      (`SceneComponent.SetVisibility` (`self.Mesh`) (not (`self.Use Skeletal Mesh?`)) false)
      (if (`self.Use Skeletal Mesh?`)
        (`PrimitiveComponent.SetCollisionEnabled` _skmesh "QueryAndPhysics")
        (`PrimitiveComponent.SetCollisionEnabled` _mesh "NoCollision")
        (else
          (`PrimitiveComponent.SetCollisionEnabled` _skmesh "NoCollision")
          (`PrimitiveComponent.SetCollisionEnabled` _mesh "QueryAndPhysics")))
      (`StaticMeshComponent.SetStaticMesh` (`self.Mesh`) (`self.Source Mesh`))
      (`SkeletalMeshComponent.SetSkeletalMeshAsset` (`self.SKMesh`) (`self.Source Skeltal Mesh`))
      (`PrimitiveComponent.SetLightingChannels` (`self.Mesh`) _bchannel0 _bchannel1 _bchannel2)
      (`PrimitiveComponent.SetLightingChannels` (`self.Niagara`) _bchannel0 _bchannel1 _bchannel2)
      (`PrimitiveComponent.SetLightingChannels` (`self.SKMesh`) _bchannel0 _bchannel1 _bchannel2))
    (:`then_1`
      ;[1 1 1] Materials Setup
      (bind _returnvalue (`KismetMaterialLibrary.CreateDynamicMaterialInstance` (select `/Game/HoloGen/Blueprints/Core/Enum_ParticleType` (`self.Pixel Type`) :`NewEnumerator0` "/Game/HoloGen/Materials/Instance/MI_Pixel_Masked.MI_Pixel_Masked" :`NewEnumerator1` "/Game/HoloGen/Materials/Instance/MI_Pixel_Transluscent.MI_Pixel_Transluscent" :`NewEnumerator2` "/Game/HoloGen/Materials/Instance/MI_Pixel_Masked.MI_Pixel_Masked" :`NewEnumerator3` "/Game/HoloGen/Materials/Instance/MI_Pixel_Transluscent.MI_Pixel_Transluscent" :!type "MaterialInterface Object Reference")))
      (bind _output_get (set `self.DynamicParticleMat` _returnvalue))
      (`MaterialInstanceDynamic.SetTextureParameterValue` _output_get "Alpha" (select `/Game/HoloGen/Blueprints/Core/Enum_ParticleType` (`self.Pixel Type`) :`NewEnumerator0` "/Game/HoloGen/Textures/Utility/T_White.T_White" :`NewEnumerator1` "/Game/HoloGen/Textures/Utility/T_Pixel_01.T_Pixel_01" :`NewEnumerator2` "/Game/HoloGen/Textures/Utility/T_Pixel_03.T_Pixel_03" :`NewEnumerator3` (`self.Custom Pixel Input`)))
      (bind _returnvalue_2 (`KismetMaterialLibrary.CreateDynamicMaterialInstance` "/Game/HoloGen/Materials/Instance/MI_String_Particle.MI_String_Particle"))
      (set `self.DynamicStringMat` _returnvalue_2)
      (bind _returnvalue_3 (`KismetMaterialLibrary.CreateDynamicMaterialInstance` (select `bool` (== (`self.Texture Style`) 10) :`false` (select `bool` (`self.Occluder Mesh?`) :`false` "/Game/HoloGen/Materials/Instance/MI_MeshMat.MI_MeshMat" :`true` "/Game/HoloGen/Materials/Instance/MI_MeshMat_Blackout.MI_MeshMat_Blackout" :!type "MaterialInterface Object Reference") :`true` (select `bool` (`self.Occluder Mesh?`) :`false` "/Game/HoloGen/Materials/Instance/MI_MeshMasked_WireFrame.MI_MeshMasked_WireFrame" :`true` "/Game/HoloGen/Materials/Instance/MI_MeshMasked_WireFrame_Blackout.MI_MeshMasked_WireFrame_Blackout" :!type "MaterialInterface Object Reference"))))
      (bind _output_get_2 (set `self.DynamicMeshMat` _returnvalue_3))
      (if (`KismetSystemLibrary.IsValid` _output_get_2)
        (`MaterialInstanceDynamic.SetTextureParameterValue` _output_get_2 "SourceColor" (`self.Mesh Color Map`))
        (`PrimitiveComponent.SetMaterial` (`self.Mesh`) 0 (`self.DynamicMeshMat`))
        (`PrimitiveComponent.SetMaterial` (`self.SKMesh`) 0 (`self.DynamicMeshMat`))
        (`KismetArrayLibrary.Array_Resize` (`self.NumMaterialSlots`) (`PrimitiveComponent.GetNumMaterials` (select `bool` (`self.Use Skeletal Mesh?`) :`false` (`self.Mesh`) :`true` (`self.SKMesh`) :!type "PrimitiveComponent Object Reference")))
        (for (_ _array_index) (`self.NumMaterialSlots`)
          (`PrimitiveComponent.SetMaterial` (`self.Mesh`) _array_index (`self.DynamicMeshMat`))
          (`PrimitiveComponent.SetMaterial` (`self.SKMesh`) _array_index (`self.DynamicMeshMat`))
          (`NiagaraComponent.SetVariableMaterial` (`self.Niagara`) "ParticleMat" (`self.DynamicParticleMat`))
          (`NiagaraComponent.SetVariableMaterial` (`self.Niagara`) "StringMat" (`self.DynamicStringMat`))
          (`MaterialInstanceDynamic.SetScalarParameterValue` (`self.DynamicMeshMat`) "Normal Map Strength" (`self.Normal Map Strength`))
          (`MaterialInstanceDynamic.SetTextureParameterValue` (`self.DynamicMeshMat`) "Normal Map" (`self.Normal Map`))
          (`MaterialInstanceDynamic.SetScalarParameterValue` (`self.DynamicMeshMat`) "Recieves Lights?" (`KismetMathLibrary.SelectFloat` 1.0 0.0 (`self.Recieves Lights?`)))
          (`MaterialInstanceDynamic.SetScalarParameterValue` (`self.DynamicStringMat`) "Recieves Lights?" (`KismetMathLibrary.SelectFloat` 1.0 0.0 (`self.Recieves Lights?`)))
          (`MaterialInstanceDynamic.SetScalarParameterValue` (`self.DynamicParticleMat`) "Recieves Lights?" (`KismetMathLibrary.SelectFloat` 1.0 0.0 (`self.Recieves Lights?`)))
          (`MaterialInstanceDynamic.SetScalarParameterValue` (`self.DynamicBlackoutMat`) "Recieves Lights?" (`KismetMathLibrary.SelectFloat` 1.0 0.0 (`self.Recieves Lights?`))))))
    (:`then_2`
      ;[1 1 1] Particle Material Parameters
      (`MaterialInstanceDynamic.SetScalarParameterValue` (`self.DynamicParticleMat`) "EmissivePower" (* (`self.Master Emissive Multiplier`) (`self.Pixel Emissive Strength`)))
      (`MaterialInstanceDynamic.SetScalarParameterValue` (`self.DynamicMeshMat`) "EmissivePower" (* (`self.Master Emissive Multiplier`) (`self.Pixel Emissive Strength`)))
      (`MaterialInstanceDynamic.SetScalarParameterValue` (`self.DynamicStringMat`) "EmissivePower" (* (`self.Master Emissive Multiplier`) (`self.Strings Emissive Strength`)))
      (`MaterialInstanceDynamic.SetScalarParameterValue` (`self.DynamicParticleMat`) "Random_Intensity" (`self.Random Color Intensity`))
      (`MaterialInstanceDynamic.SetScalarParameterValue` (`self.DynamicStringMat`) "Random_Intensity" (`self.Random Color Intensity`))
      (`FXSystemComponent.SetFloatParameter` (`self.Niagara`) "Noise_Strength" (`self.Floating Noise Intensity`))
      (`FXSystemComponent.SetFloatParameter` (`self.Niagara`) "Noise_Scale" (`self.Floating Noise Scale`)))
    (:`then_3`
      ;[1 1 1] Mesh Parameters
      (`MaterialInstanceDynamic.SetScalarParameterValue` (`self.DynamicMeshMat`) "TintLerp" (select `bool` (`self.Use Tint instead of Texture?`) :`true` 1.0))
      (`MaterialInstanceDynamic.SetScalarParameterValue` (`self.DynamicParticleMat`) "TintLerp" (select `bool` (`self.Use Tint instead of Texture?`) :`true` 1.0))
      (`MaterialInstanceDynamic.SetScalarParameterValue` (`self.DynamicStringMat`) "TintLerp" (select `bool` (`self.Use Tint instead of Texture?`) :`true` 1.0))
      (if (`self.Use Tint instead of Texture?`)
        (`MaterialInstanceDynamic.SetVectorParameterValue` (`self.DynamicStringMat`) "Tint" (`self.Color Tint`))
        (`MaterialInstanceDynamic.SetVectorParameterValue` (`self.DynamicMeshMat`) "Tint" (`self.Color Tint`))
        (`MaterialInstanceDynamic.SetVectorParameterValue` (`self.DynamicParticleMat`) "Tint" (`self.Color Tint`))
        (else
          (`MaterialInstanceDynamic.SetTextureParameterValue` (`self.DynamicParticleMat`) "Mesh_BaseColor" (`self.Mesh Color Map`))
          (`MaterialInstanceDynamic.SetTextureParameterValue` (`self.DynamicMeshMat`) "Mesh_BaseColor" (`self.Mesh Color Map`))
          (`MaterialInstanceDynamic.SetTextureParameterValue` (`self.DynamicStringMat`) "Mesh_BaseColor" (`self.Mesh Color Map`))))
      (`MaterialInstanceDynamic.SetTextureParameterValue` (`self.DynamicMeshMat`) "Mask_Material" (select `/Game/HoloGen/Blueprints/Core/Enum_TextureMat` (`self.Texture Style`) :`NewEnumerator0` "/Game/HoloGen/Textures/Utility/T_LidarAlpha_01.T_LidarAlpha_01" :`NewEnumerator1` "/Game/HoloGen/Textures/Utility/T_LidarAlpha_02.T_LidarAlpha_02" :`NewEnumerator2` "/Game/HoloGen/Textures/Utility/T_LidarAlpha_03_Sparse.T_LidarAlpha_03_Sparse" :`NewEnumerator3` "/Game/HoloGen/Textures/Utility/T_GridA-01.T_GridA-01" :`NewEnumerator4` "/Game/HoloGen/Textures/Utility/T_GridC-01.T_GridC-01" :`NewEnumerator5` "/Game/HoloGen/Textures/Utility/T_Grid_03-01.T_Grid_03-01" :`NewEnumerator8` "/Game/HoloGen/Textures/Utility/T_DotGrid_01.T_DotGrid_01" :`NewEnumerator9` "/Game/HoloGen/Textures/Utility/T_DotGrid_02.T_DotGrid_02" :`NewEnumerator10` "/Game/HoloGen/Textures/Utility/T_DotGrid_03.T_DotGrid_03" :`NewEnumerator11` "/Game/HoloGen/Textures/Utility/T_GridB-01.T_GridB-01" :`NewEnumerator12` "/Game/HoloGen/Textures/Utility/T_White.T_White" :`NewEnumerator7` (`self.Custom Texture Input`)))
      (`MaterialInstanceDynamic.SetScalarParameterValue` (`self.DynamicMeshMat`) "Mask_Scale" (`self.Texture Scale`))
      (`MaterialInstanceDynamic.SetScalarParameterValue` (`self.DynamicMeshMat`) "Use Anim Tools?" (`KismetMathLibrary.SelectFloat` 1.0 0.0 (`self.Activate Falloff Tools?`)))
      (`MaterialInstanceDynamic.SetScalarParameterValue` (`self.DynamicMeshMat`) "Opacity" (`self.Texture Opacity`))
      (`MaterialInstanceDynamic.SetScalarParameterValue` (`self.DynamicMeshMat`) "EmissivePower" (* (`self.Master Emissive Multiplier`) (`self.Texture Emissive Strength`)))
      (`MaterialInstanceDynamic.SetScalarParameterValue` (`self.DynamicMeshMat`) "Mix Noise" (`self.Noise Mix`))
      (`MaterialInstanceDynamic.SetTextureParameterValue` (`self.DynamicMeshMat`) "Noise Texture" (select `/Game/HoloGen/Blueprints/Core/Enum_MaskNoise` (`self.Noise Style`) :`NewEnumerator0` "/Game/HoloGen/Textures/Utility/T_Perlin1.T_Perlin1" :`NewEnumerator1` "/Game/HoloGen/Textures/Utility/T_5036.T_5036" :`NewEnumerator2` "/Game/HoloGen/Textures/Utility/T_MultiStreak_01.T_MultiStreak_01" :`NewEnumerator3` "/Game/HoloGen/Textures/Utility/T_SQUARES_01.T_SQUARES_01" :`NewEnumerator4` "/Game/HoloGen/Textures/Utility/T_Pintstripe_01-rotated.T_Pintstripe_01-rotated" :`NewEnumerator5` "/Game/HoloGen/Textures/Utility/T_Pintstripe_01-01.T_Pintstripe_01-01" :`NewEnumerator7` (`self.Custom Noise Input`)))
      (`MaterialInstanceDynamic.SetScalarParameterValue` (`self.DynamicMeshMat`) "Noise Texture Scale" (`self.Noise Tiling`))
      (`MaterialInstanceDynamic.SetScalarParameterValue` (`self.DynamicMeshMat`) "Noise Speed X" (`self.Noise Speed X`))
      (`MaterialInstanceDynamic.SetScalarParameterValue` (`self.DynamicMeshMat`) "Noise Speed Y" (`self.Noise Speed Y`))
      (`MaterialInstanceDynamic.SetScalarParameterValue` (`self.DynamicMeshMat`) "Blend Range" (`self.Distance Blend Softness`))
      (`MaterialInstanceDynamic.SetScalarParameterValue` (`self.DynamicMeshMat`) "Blend Scale" (`self.Distance Blend Scale`))
      (`MaterialInstanceDynamic.SetTextureParameterValue` (`self.DynamicMeshMat`) "ScanlineTex" (select `/Game/HoloGen/Blueprints/Core/Enum_ScanlineType` (`self.Scanline Type`) :`NewEnumerator0` "/Game/HoloGen/Textures/Utility/T_Line2.T_Line2" :`NewEnumerator1` "/Game/HoloGen/Textures/Utility/T_Pulse_01.T_Pulse_01" :!type "Texture Object Reference"))
      (`MaterialInstanceDynamic.SetScalarParameterValue` (`self.DynamicMeshMat`) "Fresnel Amount" (`self.Texture Fresnel Amount`)))
    (:`then_4`
      ;[1 1 1] Set Niagara Spawn Counts
      (`NiagaraComponent.SetVariableInt` (`self.Niagara`) "SpawnCount" (`self.Static Spawn Count`))
      (`NiagaraComponent.SetVariableInt` (`self.Niagara`) "Floaters_SpawnCount" (`self.Floating Spawn Count`))
      (`NiagaraComponent.SetVariableInt` (`self.Niagara`) "Strings_SpawnCount" (`self.Strings Spawn Count`)))
    (:`then_5`
      ;[1 1 1] Set Niagara Particle Sizes
      (`NiagaraComponent.SetVariableFloat` (`self.Niagara`) "StaticSize_Min" (`self.PixelTypeSwitchbox` (`self.Static Min Scale`)))
      (`NiagaraComponent.SetVariableFloat` (`self.Niagara`) "StaticSize_Max" (`self.PixelTypeSwitchbox` (`self.Static Max Scale`)))
      (`NiagaraComponent.SetVariableFloat` (`self.Niagara`) "FloaterSize_Min" (`self.PixelTypeSwitchbox` (`self.Floating Min Scale`)))
      (`NiagaraComponent.SetVariableFloat` (`self.Niagara`) "FloaterSize_Max" (`self.PixelTypeSwitchbox` (`self.Floating Max Scale`)))
      (`NiagaraComponent.SetVariableFloat` (`self.Niagara`) "Floater_Speed" (`self.Floating Speed`))
      (`NiagaraComponent.SetVariableFloat` (`self.Niagara`) "StringsSize_Min" (`self.Strings Min Scale`))
      (`NiagaraComponent.SetVariableFloat` (`self.Niagara`) "StringsSize_Max" (`self.Strings Max Scale`)))
    (:`then_6`
      ;[1 1 1] Set Niagara Variables
      (`NiagaraComponent.SetVariableFloat` (`self.Niagara`) "Randomize" (`self.RandomOffset`))
      (`PrimitiveComponent.SetCastShadow` (`self.Niagara`) (`self.Particles Cast Shadow?`)))
    (:`then_7`
      ;[1 1 1] Extra
      (`PrimitiveComponent.SetBoundsScale` (`self.Niagara`) (`self.Bounds Scale`))
      (`SceneComponent.SetVisibility` (`self.Mesh`) (and (`self.Mesh Visible?`) (not (`self.Use Skeletal Mesh?`))) false)
      (`SceneComponent.SetVisibility` (`self.SKMesh`) (and (`self.Mesh Visible?`) (`self.Use Skeletal Mesh?`)) false))
    (:`then_8`
      ;[1 1 1] Glitching
      (`MaterialInstanceDynamic.SetScalarParameterValue` (`self.DynamicMeshMat`) "Glitch Distortion" (`self.Bad Reception`))
      (`MaterialInstanceDynamic.SetScalarParameterValue` (`self.DynamicMeshMat`) "Scanline Distortion Intensity" (`self.ScanLines Distortion Intensity`))
      (`MaterialInstanceDynamic.SetScalarParameterValue` (`self.DynamicMeshMat`) "San Line Intensity" (`self.Scanline Brightness`))
      (`MaterialInstanceDynamic.SetScalarParameterValue` (`self.DynamicMeshMat`) "Sanline Speed" (`self.Scanline Speed`))
      (`MaterialInstanceDynamic.SetScalarParameterValue` (`self.DynamicMeshMat`) "Scanline Scale" (`self.Scanline Scale`)))
    (:`then_9`
      ;[1 1 1] Animation
      (`self.FalloffUpdate`))))