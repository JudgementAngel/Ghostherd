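; BP_HolographicTree is a test-case actor that dresses a holographic tree effect from layered meshes: base, hologram, wireframe, two ray lines and a horizontal-line (HLine) mesh.
; Its construction script calls the SetMeshMaterial macro per mesh, which creates a dynamic material instance and assigns it to every material slot.
; Both ray-line materials receive a RayPosition parameter from their configured offset plus the actor's location.
; The event graph holds no active logic.
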(fn `UserConstructionScript`
  (bind (_x _y _z) (`KismetMathLibrary.BreakVector3f` (+ (`self.RayPositon1`) (`self.K2_GetActorLocation`))))
  (bind (_x_2 _y_2 _z_2) (`KismetMathLibrary.BreakVector3f` (+ (`self.RayPositon2`) (`self.K2_GetActorLocation`))))
  (`self.SetMeshMaterial` (`self.M_Base`) (`self.BaseMesh`)
    (:`Completed`
      (`self.SetMeshMaterial` (`self.M_Holo`) (`self.Holo`)
        (:`Completed`
          (`self.SetMeshMaterial` (`self.M_Wireframe`) (`self.Wireframe`)
            (:`Completed`
              (bind _dynamicmaterial (`self.SetMeshMaterial` (`self.M_RayLine`) (`self.RayLine1`))
                (:`LoopBody`
                  (`MaterialInstanceDynamic.SetVectorParameterValue` _dynamicmaterial "RayPosition" (make `LinearColor` _x _y _z 1.0)))
                (:`Completed`
                  (bind _dynamicmaterial_2 (`self.SetMeshMaterial` (`self.M_RayLine`) (`self.RayLine2`))
                    (:`LoopBody`
                      (`MaterialInstanceDynamic.SetVectorParameterValue` _dynamicmaterial_2 "RayPosition" (make `LinearColor` _x_2 _y_2 _z_2 1.0)))
                    (:`Completed`
                      (`self.SetMeshMaterial` (`self.M_HLine`) (`self.HLine`)))))))))))))