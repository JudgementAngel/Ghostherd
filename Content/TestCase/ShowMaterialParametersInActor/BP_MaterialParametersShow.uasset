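; Test actor that exposes a material instance's parameters on the actor and applies them to its Cube mesh.
; GenerateParameterList creates a dynamic instance from BaseMaterialInstance, assigns it to the Cube, then rebuilds name arrays and name-to-value maps from its vector, texture and scalar overrides.
; The construction script pushes those map values back into the dynamic instance, so changes to the maps show on construction.
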(fn `GenerateParameterList`
  (bind _basematerialinstance (`self.BaseMaterialInstance`))
  (bind _returnvalue (`KismetMaterialLibrary.CreateDynamicMaterialInstance` (`self.BaseMaterialInstance`)))
  (set `self.MaterialInstanceDynamic` _returnvalue)
  (`PrimitiveComponent.SetMaterial` (`self.Cube`) 0 (`self.MaterialInstanceDynamic`))
  (`BlueprintMapLibrary.Map_Clear` (`self.VectorParameters`))
  (`BlueprintMapLibrary.Map_Clear` (`self.ScalarParameters`))
  (`BlueprintMapLibrary.Map_Clear` (`self.TextureParameters`))
  (`KismetArrayLibrary.Array_Clear` (`self.ScalarParameterNames`))
  (`KismetArrayLibrary.Array_Clear` (`self.VectorParameterNames`))
  (`KismetArrayLibrary.Array_Clear` (`self.TextureParameterNames`))
  (`|ExecutionSequence`
    (:`then_0`
      (for (_array_element _array_index) (`MaterialInstance.VectorParameterValues` _basematerialinstance)
        (bind _name (break `MaterialParameterInfo` (break `VectorParameterValue` _array_element)))
        (`BlueprintMapLibrary.Map_Add` (`self.VectorParameters`) _name (`.ParameterValue` (break `VectorParameterValue` _array_element)))
        (`KismetArrayLibrary.Array_Set` (`self.VectorParameterNames`) _array_index _name true)))
    (:`then_1`
      (for (_array_element_2 _array_index_2) (`MaterialInstance.TextureParameterValues` _basematerialinstance)
        (bind _name_2 (break `MaterialParameterInfo` (break `TextureParameterValue` _array_element_2)))
        (`BlueprintMapLibrary.Map_Add` (`self.TextureParameters`) _name_2 (`.ParameterValue` (break `TextureParameterValue` _array_element_2)))
        (`KismetArrayLibrary.Array_Set` (`self.TextureParameterNames`) _array_index_2 _name_2 true)))
    (:`then_2`
      (for (_array_element_3 _array_index_3) (`MaterialInstance.ScalarParameterValues` _basematerialinstance)
        (bind _name_3 (break `MaterialParameterInfo` (break `ScalarParameterValue` _array_element_3)))
        (`BlueprintMapLibrary.Map_Add` (`self.ScalarParameters`) _name_3 (`.ParameterValue` (break `ScalarParameterValue` _array_element_3)))
        (`KismetArrayLibrary.Array_Set` (`self.ScalarParameterNames`) _array_index_3 _name_3 true)))))

(fn `UserConstructionScript`
  (`/Engine/EditorBlueprintResources/StandardMacros.IsValid` (`self.MaterialInstanceDynamic`)
    (:`Is Valid`
      (`|ExecutionSequence`
        (:`then_0`
          (for _array_element (`self.VectorParameterNames`)
            (bind (_value _returnvalue) (`BlueprintMapLibrary.Map_Find` (`self.VectorParameters`) _array_element))
            (if _returnvalue
              (`MaterialInstanceDynamic.SetVectorParameterValue` (`self.MaterialInstanceDynamic`) _array_element _value))))
        (:`then_1`
          (for _array_element_2 (`self.TextureParameterNames`)
            (bind (_value_2 _returnvalue_2) (`BlueprintMapLibrary.Map_Find` (`self.TextureParameters`) _array_element_2))
            (if _returnvalue_2
              (`MaterialInstanceDynamic.SetTextureParameterValue` (`self.MaterialInstanceDynamic`) _array_element_2 _value_2))))
        (:`then_2`
          (for _array_element_3 (`self.ScalarParameterNames`)
            (bind (_value_3 _returnvalue_3) (`BlueprintMapLibrary.Map_Find` (`self.ScalarParameters`) _array_element_3))
            (if _returnvalue_3
              (`MaterialInstanceDynamic.SetScalarParameterValue` (`self.MaterialInstanceDynamic`) _array_element_3 _value_3))))))))