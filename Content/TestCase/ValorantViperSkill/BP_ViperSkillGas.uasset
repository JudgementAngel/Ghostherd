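; Test actor for a Valorant Viper-style gas skill that expands a bone-controlled mesh to fit the surrounding space.
; BeginPlay line-traces along each control direction, storing the hit or trace end as that point's target.
; Tick eases each point toward its target with fixed-step VInterpTo and writes actor-relative offsets into the cube skeleton's AnimBP bone control variables.
; Debug spheres show targets and moving points; surroundings are sampled only once.
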(event `self.ReceiveBeginPlay`
  (bind _returnvalue_location (`KismetMathLibrary.BreakTransform` (`self.GetTransform`)))
  (`|ExecutionSequence`
    (:`then_0`
      (for (_array_element _array_index) (`self.CtrlList`)
        (bind _returnvalue (`KismetMathLibrary.Normal` _array_element))
        (bind (_outhit _returnvalue_2) (`KismetSystemLibrary.LineTraceSingle` :`Start` (+ _returnvalue_location (* _returnvalue (`self.RayStart`))) :`End` (+ _returnvalue_location (* _returnvalue (`self.RayEnd`))) :`TraceChannel` "TraceTypeQuery1" :`DrawDebugType` "ForDuration"))
        (bind _returnvalue_3 (`KismetMathLibrary.SelectVector` (`.Location` (`GameplayStatics.BreakHitResult` _outhit)) (`.TraceEnd` (`GameplayStatics.BreakHitResult` _outhit)) _returnvalue_2))
        (`KismetArrayLibrary.Array_Set` (`self.CtrlTargetList`) _array_index _returnvalue_3)
        (`KismetArrayLibrary.Array_Set` (`self.CtrlList_Current`) _array_index (+ _returnvalue_location (* _returnvalue (`self.InitLength`))))
        (`KismetSystemLibrary.DrawDebugSphere` _returnvalue_3 3.0 12 (struct :`R` 0.200514 :`G` 1.0 :`A` 1.0) 10.0)
        (if _returnvalue_2
          _)))
    (:`then_1`
      (bind _ascube_with_bone_skeleton_anim_blueprint (cast `/Game/TestCase/ValorantViperSkill/CubeWithBone_Skeleton_AnimBlueprint` (`SkeletalMeshComponent.GetAnimInstance` (`self.SkeletalMesh`))))
      (set `self.AnimInstance` _ascube_with_bone_skeleton_anim_blueprint))))

(event `self.ReceiveTick`
  (params (DeltaSeconds :type "Float (single-precision)"))
  (bind _returnvalue_location (`KismetMathLibrary.BreakTransform` (`self.GetTransform`)))
  (bind _animinstance (`self.AnimInstance`))
  (bind _animinstance_2 (`self.AnimInstance`))
  (bind _animinstance_3 (`self.AnimInstance`))
  (`|ExecutionSequence`
    (:`then_0`
      (for (_array_element _array_index) (`self.CtrlList_Current`)
        (bind _returnvalue (`KismetMathLibrary.VInterpTo` _array_element (`|GetArrayItem` (`self.CtrlTargetList`) _array_index) 0.05 0.1))
        (`KismetArrayLibrary.Array_Set` (`self.CtrlList_Current`) _array_index _returnvalue)
        (`KismetSystemLibrary.DrawDebugSphere` _returnvalue 5.0 3 (struct :`R` 0.150133 :`G` 0.015625 :`B` 1.0 :`A` 1.0))
        (switch `int` _array_index
          (:`0`
            (bind _returnvalue_2 (- _returnvalue _returnvalue_location))
            (set `/Game/TestCase/ValorantViperSkill/CubeWithBone_Skeleton_AnimBlueprint.Bone 0 Ctrl Location` _returnvalue_2 _animinstance_2))
          (:`1`
            (set `/Game/TestCase/ValorantViperSkill/CubeWithBone_Skeleton_AnimBlueprint.Bone 00 Ctrl Location` _returnvalue_2 _animinstance_2))
          (:`2`
            (set `/Game/TestCase/ValorantViperSkill/CubeWithBone_Skeleton_AnimBlueprint.Bone 01 Ctrl Location` _returnvalue_2 _animinstance_2))
          (:`3`
            (set `/Game/TestCase/ValorantViperSkill/CubeWithBone_Skeleton_AnimBlueprint.Bone 02 Ctrl Location` _returnvalue_2 _animinstance_2))
          (:`4`
            (set `/Game/TestCase/ValorantViperSkill/CubeWithBone_Skeleton_AnimBlueprint.Bone 03 Ctrl Location` _returnvalue_2 _animinstance_2))
          (:`5`
            (set `/Game/TestCase/ValorantViperSkill/CubeWithBone_Skeleton_AnimBlueprint.Bone 04 Ctrl Location` _returnvalue_2 _animinstance_2))
          (:`6`
            (set `/Game/TestCase/ValorantViperSkill/CubeWithBone_Skeleton_AnimBlueprint.Bone 05 Ctrl Location` _returnvalue_2 _animinstance_2))
          (:`7`
            (set `/Game/TestCase/ValorantViperSkill/CubeWithBone_Skeleton_AnimBlueprint.Bone 06 Ctrl Location` _returnvalue_2 _animinstance_2))
          (:`8`
            (set `/Game/TestCase/ValorantViperSkill/CubeWithBone_Skeleton_AnimBlueprint.Bone 07 Ctrl Location` _returnvalue_2 _animinstance_2))
          (:`9`
            (set `/Game/TestCase/ValorantViperSkill/CubeWithBone_Skeleton_AnimBlueprint.Bone 10 Ctrl Location` _returnvalue_2 _animinstance))
          (:`10`
            (set `/Game/TestCase/ValorantViperSkill/CubeWithBone_Skeleton_AnimBlueprint.Bone 11 Ctrl Location` _returnvalue_2 _animinstance))
          (:`11`
            (set `/Game/TestCase/ValorantViperSkill/CubeWithBone_Skeleton_AnimBlueprint.Bone 12 Ctrl Location` _returnvalue_2 _animinstance))
          (:`12`
            (set `/Game/TestCase/ValorantViperSkill/CubeWithBone_Skeleton_AnimBlueprint.Bone 13 Ctrl Location` _returnvalue_2 _animinstance))
          (:`13`
            (set `/Game/TestCase/ValorantViperSkill/CubeWithBone_Skeleton_AnimBlueprint.Bone 14 Ctrl Location` _returnvalue_2 _animinstance))
          (:`14`
            (set `/Game/TestCase/ValorantViperSkill/CubeWithBone_Skeleton_AnimBlueprint.Bone 15 Ctrl Location` _returnvalue_2 _animinstance))
          (:`15`
            (set `/Game/TestCase/ValorantViperSkill/CubeWithBone_Skeleton_AnimBlueprint.Bone 16 Ctrl Location` _returnvalue_2 _animinstance))
          (:`16`
            (set `/Game/TestCase/ValorantViperSkill/CubeWithBone_Skeleton_AnimBlueprint.Bone 17 Ctrl Location` _returnvalue_2 _animinstance))
          (:`17`
            (set `/Game/TestCase/ValorantViperSkill/CubeWithBone_Skeleton_AnimBlueprint.Bone 2 Ctrl Location` _returnvalue_2 _animinstance_3))
          (:`18`
            (set `/Game/TestCase/ValorantViperSkill/CubeWithBone_Skeleton_AnimBlueprint.Bone 20 Ctrl Location` _returnvalue_2 _animinstance_3))
          (:`19`
            (set `/Game/TestCase/ValorantViperSkill/CubeWithBone_Skeleton_AnimBlueprint.Bone 21 Ctrl Location` _returnvalue_2 _animinstance_3))
          (:`20`
            (set `/Game/TestCase/ValorantViperSkill/CubeWithBone_Skeleton_AnimBlueprint.Bone 22 Ctrl Location` _returnvalue_2 _animinstance_3))
          (:`21`
            (set `/Game/TestCase/ValorantViperSkill/CubeWithBone_Skeleton_AnimBlueprint.Bone 23 Ctrl Location` _returnvalue_2 _animinstance_3))
          (:`22`
            (set `/Game/TestCase/ValorantViperSkill/CubeWithBone_Skeleton_AnimBlueprint.Bone 24 Ctrl Location` _returnvalue_2 _animinstance_3))
          (:`23`
            (set `/Game/TestCase/ValorantViperSkill/CubeWithBone_Skeleton_AnimBlueprint.Bone 25 Ctrl Location` _returnvalue_2 _animinstance_3))
          (:`24`
            (set `/Game/TestCase/ValorantViperSkill/CubeWithBone_Skeleton_AnimBlueprint.Bone 26 Ctrl Location` _returnvalue_2 _animinstance_3))
          (:`25`
            (set `/Game/TestCase/ValorantViperSkill/CubeWithBone_Skeleton_AnimBlueprint.Bone 27 Ctrl Location` _returnvalue_2 _animinstance_3)))))))

(fn `UserConstructionScript`)