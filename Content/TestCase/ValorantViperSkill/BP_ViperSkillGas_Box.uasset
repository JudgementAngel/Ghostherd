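; Test actor recreating Valorant Viper's gas skill as a box skeletal mesh that expands to fit its surroundings.
; On BeginPlay it line-traces along each CtrlList direction from the actor, storing hit or end points as targets and initial points as current positions.
; Each Tick interpolates current points toward targets with fixed steps and writes actor-relative offsets into the AnimBlueprint's CtrlList.
; Debug traces and spheres visualize the points.
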(event `self.ReceiveBeginPlay`
  (bind _returnvalue_location (`KismetMathLibrary.BreakTransform` (`self.GetTransform`)))
  (`|ExecutionSequence`
    (:`then_0`
      (for (_array_element _array_index) (`self.CtrlList`)
        (bind _returnvalue (`KismetMathLibrary.Normal` _array_element))
        (bind (_outhit _returnvalue_2) (`KismetSystemLibrary.LineTraceSingle` :`Start` (+ _returnvalue_location (* _returnvalue (`self.RayStart`))) :`End` (+ _returnvalue_location (* _returnvalue (`self.RayEnd`))) :`TraceChannel` "TraceTypeQuery1" :`DrawDebugType` "ForDuration"))
        (bind _returnvalue_3 (`KismetMathLibrary.SelectVector` (`.Location` (`GameplayStatics.BreakHitResult` _outhit)) (`.TraceEnd` (`GameplayStatics.BreakHitResult` _outhit)) _returnvalue_2))
        (`KismetArrayLibrary.Array_Set` (`self.CtrlTargetList`) _array_index _returnvalue_3)
        (`KismetArrayLibrary.Array_Set` (`self.CtrlList_Current`) _array_index (+ _returnvalue_location (* _returnvalue (`self.InitLength`))))
        (`KismetSystemLibrary.DrawDebugSphere` _returnvalue_3 3.0 12 (struct :`R` 0.200514 :`G` 1.0 :`A` 1.0) 10.0)
        (if _returnvalue_2
          _)))
    (:`then_1`
      (bind _asviper_box_skeleton_anim_blueprint (cast `/Game/TestCase/ValorantViperSkill/ViperBox_Skeleton_AnimBlueprint` (`SkeletalMeshComponent.GetAnimInstance` (`self.SkeletalMesh`))))
      (set `self.As Viper Box Skeleton Anim Blueprint` _asviper_box_skeleton_anim_blueprint))))

(event `self.ReceiveTick`
  (params (DeltaSeconds :type "Float (single-precision)"))
  (bind _returnvalue_location (`KismetMathLibrary.BreakTransform` (`self.GetTransform`)))
  (`|ExecutionSequence`
    (:`then_0`
      (for (_array_element _array_index) (`self.CtrlList_Current`)
        (bind _returnvalue (`KismetMathLibrary.VInterpTo` _array_element (`|GetArrayItem` (`self.CtrlTargetList`) _array_index) 0.05 0.1))
        (`KismetArrayLibrary.Array_Set` (`self.CtrlList_Current`) _array_index _returnvalue)
        (`KismetSystemLibrary.DrawDebugSphere` _returnvalue 5.0 3 (struct :`R` 0.150133 :`G` 0.015625 :`B` 1.0 :`A` 1.0))
        (`KismetArrayLibrary.Array_Set` (`/Game/TestCase/ValorantViperSkill/ViperBox_Skeleton_AnimBlueprint.CtrlList` (`self.As Viper Box Skeleton Anim Blueprint`)) _array_index (- _returnvalue _returnvalue_location))))))

(fn `UserConstructionScript`)