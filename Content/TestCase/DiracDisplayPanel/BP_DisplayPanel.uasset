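; Display panel actor that animates a dynamic material on its Plane, cycling endlessly through three display states with four running digit counters.
; BeginPlay creates the material, then loops two timelines with delays: one ramps Character_BlockIntensity, the State switches, and the other ramps it back.
; The middle state skips that ramp-back and uses a slower StateSequenceSpeed.
; Tick advances four counters at different rates, feeding their wrapped 0–9 digits to the material.
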(event `self.ReceiveBeginPlay`
  (bind _plane (`self.Plane`))
  (`|ExecutionSequence`
    (:`then_0`
      (bind _returnvalue (`PrimitiveComponent.CreateDynamicMaterialInstance` _plane 0 (`PrimitiveComponent.GetMaterial` _plane 0) "None"))
      (bind _output_get (set `self.DynamicMat` _returnvalue))
      (`PrimitiveComponent.SetMaterial` (`self.Plane`) 0 _output_get)
      (set `self.Index` 0)
      (`MaterialInstanceDynamic.SetScalarParameterValue` (`self.DynamicMat`) "State" (`KismetMathLibrary.Conv_IntToDouble` (mod (`self.Index`) 3)))
      (`MaterialInstanceDynamic.SetScalarParameterValue` (`self.DynamicMat`) "StateSequenceSpeed" 0.8)
      (set `self.Index` (+ (`self.Index`) 1)))
    (:`then_1`
      (`KismetSystemLibrary.Delay` 1.0 :!label _label)
      (bind (_direction _up) (`Timeline|Character_BlockIntensity_In` :!via `PlayFromStart`)
        (:`Update`
          (`MaterialInstanceDynamic.SetScalarParameterValue` (`self.DynamicMat`) "Character_BlockIntensity" _up))
        (:`Finished`
          (`MaterialInstanceDynamic.SetScalarParameterValue` (`self.DynamicMat`) "State" (`KismetMathLibrary.Conv_IntToDouble` (mod (`self.Index`) 3)))
          (bind (_direction_2 _down) (`Timeline|Character_BlockIntensity_Out` :!via `PlayFromStart`)
            (:`Update`
              (if (!= (mod (`self.Index`) 3) 1)
                (`MaterialInstanceDynamic.SetScalarParameterValue` (`self.DynamicMat`) "Character_BlockIntensity" _down)
                (`MaterialInstanceDynamic.SetScalarParameterValue` (`self.DynamicMat`) "StateSequenceSpeed" 1.0)
                (else
                  (`MaterialInstanceDynamic.SetScalarParameterValue` (`self.DynamicMat`) "StateSequenceSpeed" 0.8))))
            (:`Finished`
              (set `self.Index` (+ (`self.Index`) 1))
              (`KismetSystemLibrary.Delay` 3.0)
              (goto _label))))))))

(event `self.ReceiveTick`
  (params (DeltaSeconds :type "Float (single-precision)"))
  (`|ExecutionSequence`
    (:`then_0`
      (set `self.Number1` (+ (* DeltaSeconds 1.0) (`self.Number1`)))
      (set `self.Number2` (+ (* DeltaSeconds 2.0) (`self.Number2`)))
      (set `self.Number3` (+ (* DeltaSeconds 3.0) (`self.Number3`)))
      (set `self.Number4` (+ (* DeltaSeconds 4.0) (`self.Number4`))))
    (:`then_1`
      (`MaterialInstanceDynamic.SetScalarParameterValue` (`self.DynamicMat`) "Num1" (`KismetMathLibrary.Conv_IntToDouble` (mod (`KismetMathLibrary.FFloor` (`self.Number1`)) 10)))
      (`MaterialInstanceDynamic.SetScalarParameterValue` (`self.DynamicMat`) "Num2" (`KismetMathLibrary.Conv_IntToDouble` (mod (`KismetMathLibrary.FFloor` (`self.Number2`)) 10)))
      (`MaterialInstanceDynamic.SetScalarParameterValue` (`self.DynamicMat`) "Num3" (`KismetMathLibrary.Conv_IntToDouble` (mod (`KismetMathLibrary.FFloor` (`self.Number3`)) 10)))
      (`MaterialInstanceDynamic.SetScalarParameterValue` (`self.DynamicMat`) "Num4" (`KismetMathLibrary.Conv_IntToDouble` (mod (`KismetMathLibrary.FFloor` (`self.Number4`)) 10))))))

(fn `UserConstructionScript`)