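; Test-case actor that animates a dissolve effect on a configured set of static mesh actors when play begins.
; It creates dynamic material instances for every material on each mapped actor, storing each with that actor's min/max range and setting the dissolve parameter to the range start.
; A timeline then plays, interpolating the named scalar parameter on every stored instance between its own start and end values.
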(event `self.ReceiveBeginPlay`
  (bind _dymat_dissolveminmax (`self.DyMat_DissolveMinMax`))
  (`|ExecutionSequence`
    (:`then_0`
      (bind _keys (`BlueprintMapLibrary.Map_Keys` (`self.CtrlActor_DissolveMinMax`)))
      (for _array_element _keys
        (bind _staticmeshcomponent (`StaticMeshActor.StaticMeshComponent` _array_element))
        (for (_array_element_2 _array_index) (`MeshComponent.GetMaterials` _staticmeshcomponent)
          (bind _returnvalue (`KismetMaterialLibrary.CreateDynamicMaterialInstance` _array_element_2))
          (`PrimitiveComponent.SetMaterial` _staticmeshcomponent _array_index _returnvalue)
          (bind _value (`BlueprintMapLibrary.Map_Find` (`self.CtrlActor_DissolveMinMax`) _array_element))
          (`BlueprintMapLibrary.Map_Add` (`self.DyMat_DissolveMinMax`) _returnvalue _value)
          (`MaterialInstanceDynamic.SetScalarParameterValue` _returnvalue (`self.DissolveParameterName`) (`KismetMathLibrary.BreakVector2D` _value)))))
    (:`then_1`
      (bind (_direction _dissolve) (`Timeline|DissolveTimeline`)
        (:`Update`
          (bind _keys_2 (`BlueprintMapLibrary.Map_Keys` _dymat_dissolveminmax))
          (for _array_element_3 _keys_2
            (bind (_x _y) (`KismetMathLibrary.BreakVector2D` (`BlueprintMapLibrary.Map_Find` _dymat_dissolveminmax _array_element_3)))
            (`MaterialInstanceDynamic.SetScalarParameterValue` _array_element_3 (`self.DissolveParameterName`) (`KismetMathLibrary.Lerp` _x _y _dissolve))))))))

(fn `UserConstructionScript`)