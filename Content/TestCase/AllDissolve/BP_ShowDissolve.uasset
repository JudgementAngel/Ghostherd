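; Showcase actor that previews a dissolve material on plane, cube and sphere meshes, labeled with the material's name.
; Construction creates dynamic instances of the dissolve material and a debug input material, assigns them, and toggles debug mesh and sphere center visibility.
; On play, a timeline drives the dissolve parameter between min and max values.
; Optionally, a second timeline moves SphereCenter and feeds its world position to both materials' dissolve sphere center.
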(event `self.ReceiveBeginPlay`
  (`|ExecutionSequence`
    (:`then_0`
      (bind (_direction _dissolve) (`Timeline|Timeline`)
        (:`Update`
          (`MaterialInstanceDynamic.SetScalarParameterValue` (`self.DyMat`) (`self.DissolveParameterName`) (`KismetMathLibrary.Lerp` (`self.MinDissolveValue`) (`self.MaxDissolveValue`) _dissolve)))))
    (:`then_1`
      (if (`self.UseWorldSpaceSphereCenter`)
        (bind (_direction_2 _locationz) (`Timeline|Timeline_0`)
          (:`Update`
            (`SceneComponent.K2_SetRelativeLocation` (`self.SphereCenter`) (`KismetMathLibrary.MakeVector` 0.0 100.0 (`KismetMathLibrary.Lerp` 100.0 -300.0 _locationz)) false false)
            (`MaterialInstanceDynamic.SetVectorParameterValue` (`self.DyMat`) "DissolveSphere_Center" (`KismetMathLibrary.Conv_VectorToLinearColor` (`SceneComponent.K2_GetComponentLocation` (`self.SphereCenter`))))
            (`MaterialInstanceDynamic.SetVectorParameterValue` (`self.DyMatInput`) "DissolveSphere_Center" (`KismetMathLibrary.Conv_VectorToLinearColor` (`SceneComponent.K2_GetComponentLocation` (`self.SphereCenter`))))))))))

(fn `UserConstructionScript`
  (`|ExecutionSequence`
    (:`then_0`
      (`SceneComponent.SetVisibility` (`self.Cube_Input`) (`self.ShowDebugDissolveInput`) false)
      (`SceneComponent.SetVisibility` (`self.Sphere_Input`) (`self.ShowDebugDissolveInput`) false)
      (`SceneComponent.SetVisibility` (`self.Plane_Input`) (`self.ShowDebugDissolveInput`) false))
    (:`then_1`
      (bind _returnvalue (`KismetMaterialLibrary.CreateDynamicMaterialInstance` (`self.DissolveMat`)))
      (bind _output_get (set `self.DyMat` _returnvalue))
      (`PrimitiveComponent.SetMaterial` (`self.Plane`) 0 _output_get)
      (`PrimitiveComponent.SetMaterial` (`self.Cube`) 0 _output_get)
      (`PrimitiveComponent.SetMaterial` (`self.Sphere`) 0 _output_get))
    (:`then_2`
      (bind _returnvalue_2 (`KismetMaterialLibrary.CreateDynamicMaterialInstance` (`self.DissolveInputDebugMat`)))
      (bind _output_get_2 (set `self.DyMatInput` _returnvalue_2))
      (`PrimitiveComponent.SetMaterial` (`self.Cube_Input`) 0 _output_get_2)
      (`PrimitiveComponent.SetMaterial` (`self.Sphere_Input`) 0 _output_get_2)
      (`PrimitiveComponent.SetMaterial` (`self.Plane_Input`) 0 _output_get_2))
    (:`then_3`
      (`SceneComponent.SetVisibility` (`self.SphereCenter`) (`self.UseWorldSpaceSphereCenter`) false))
    (:`then_4`
      (`TextRenderComponent.K2_SetText` (`self.TextRender`) (`KismetTextLibrary.Conv_StringToText` (`KismetStringLibrary.Replace` (`KismetSystemLibrary.GetDisplayName` (`self.DissolveMat`)) "MI_"))))))