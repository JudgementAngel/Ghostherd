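; BP_Hero05 is the attacker in an IK test of a choke slam on a target BP_Hero04 victim.
; BeginPlay caches the victim and its own Hero_ChokeSlam_Att anim instance.
; Each Tick sets that instance's IK effector to the victim's grip socket plus a fixed offset.
; It also drives the victim's neck control from the attacker's right-hand grip socket, adjusted by offsets with X and Y negated.
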(event `self.ReceiveBeginPlay`
  (bind _asbp_hero_04 (cast `/Game/TestCase/IKAnim/BP_Hero04` (`self.Target_Vic`)))
  (set `self.As BP Hero 04` _asbp_hero_04)
  (bind _ashero_choke_slam_att (cast `/Game/TestCase/IKAnim/Hero_ChokeSlam_Att` (`SkeletalMeshComponent.GetAnimInstance` (`self.SKM_Manny`))))
  (set `self.As Hero Choke Slam Att` _ashero_choke_slam_att))

(event `self.ReceiveTick`
  (params (DeltaSeconds :type "Float (single-precision)"))
  (set `/Game/TestCase/IKAnim/Hero_ChokeSlam_Att.Effector Location` (+ (`SceneComponent.GetSocketLocation` (`/Game/TestCase/IKAnim/BP_Hero04.SK_Mannequin` (`self.As BP Hero 04`)) "ChokeSlamGripPoint") (0.0 127.08187 0.0)) (`self.As Hero Choke Slam Att`))
  (set `/Game/TestCase/IKAnim/BP_Hero04.Neck Ctrl Location` (`KismetMathLibrary.MakeVector` (* (.x (- (+ (`SceneComponent.GetSocketLocation` (`self.SKM_Manny`) "hand_r_grip") (`/Game/TestCase/IKAnim/BP_Hero04.GripOffset` (`self.As BP Hero 04`))) (0.0 5.876 156.422))) -1.0) (* (.y (- (+ (`SceneComponent.GetSocketLocation` (`self.SKM_Manny`) "hand_r_grip") (`/Game/TestCase/IKAnim/BP_Hero04.GripOffset` (`self.As BP Hero 04`))) (0.0 5.876 156.422))) -1.0) (.z (- (+ (`SceneComponent.GetSocketLocation` (`self.SKM_Manny`) "hand_r_grip") (`/Game/TestCase/IKAnim/BP_Hero04.GripOffset` (`self.As BP Hero 04`))) (0.0 5.876 156.422)))) (`self.As BP Hero 04`)))

(fn `UserConstructionScript`)