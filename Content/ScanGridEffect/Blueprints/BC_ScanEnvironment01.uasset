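; Character component that toggles an environment scan effect on IA_Scan, with optional camera shakes and start, pulse, loop and end sounds.
; A tick-driven fade state machine advances normalized time, shapes post-process blend weight through an optional curve and feeds MPC_Scan.
; It spawns BP_ScanSpwan on demand for the post-process material and optional grid-snapped Niagara grid following the character.
; Full fade-out destroys that actor and stops ticking until the next scan.
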(event `StartPulseSound`
  ;[0.000555 0 1] Pulse Sounds
  (`KismetSystemLibrary.Delay` (`self.LoopStartDelay`))
  (if (`self.IsActivated?`)
    (bind _returnvalue (`GameplayStatics.SpawnSoundAtLocation` (`self.Pulse Sound`) (`self.Current Location`) (struct) 1.0 (`self.Pulse Volume`) 0.0 (`self.Attenuation Settings`) null :!label _label))
    (set `self.PulseSoundRef` _returnvalue)
    (if (`self.IsActivated?`)
      (`KismetSystemLibrary.Delay` (`self.SoundTimeDelay`))
      (goto _label)
      (else
        (`AudioComponent.FadeOut` (`self.PulseSoundRef`) (`self.Alpha`) 0.0 "Linear")))))

(event `Play CameraShake-StartEffect`
  ;[0.1329 0 1] Camera Shake
  (if (`self.UseCameraShake?`)
    (`PlayerCameraManager.StartCameraShake` :`self` (`GameplayStatics.GetPlayerCameraManager` 0) :`ShakeClass` (`self.1-Camera Shake Start Effect`) :`Scale` (`self.1-Scale`))))

(event `EnhancedInput|/Game/ScanGridEffect/Inputs/IA_Scan`
  (params (ActionValue :type Boolean) (ElapsedSeconds :type "Float (double-precision)") (TriggeredSeconds :type "Float (double-precision)") (InputAction :type "InputAction Object Reference" :default "/Game/ScanGridEffect/Inputs/IA_Scan.IA_Scan"))
  ;[1 0.396 0.849] Controller Fade In / Fade Out:
  (:`Started`
    (`/Engine/EditorBlueprintResources/StandardMacros.DoOnce` false :!label _label_2
      (:`Completed`
        (`/Engine/EditorBlueprintResources/StandardMacros.FlipFlop`
          (:`A`
            (`self.StartScan`)
            (`self.Play CameraShake-StartEffect`)
            (set `self.IsActivated?` true)
            (`self.StartSound`)
            (`self.LoopSound`))
          (:`B`
            (`self.EndScan`)
            (`self.Play CameraShake-StopEffect`)
            (set `self.IsActivated?` false)
            (`self.EndSound`))))))
  (:`Completed`
    (goto _label_2 :!via `Reset`)))

(event `Play CameraShake-StopEffect`
  ;[0.1329 0 1] Camera Shake
  (if (`self.UseCameraShake?`)
    (`PlayerCameraManager.StartCameraShake` :`self` (`GameplayStatics.GetPlayerCameraManager` 0) :`ShakeClass` (`self.2-Camera Shake Stop Effect`) :`Scale` (`self.2-Scale`))))

(event `LoopSound`
  (bind _current_location (`self.Current Location`))
  (bind _loopsoundref (`self.LoopSoundRef`))
  ;[0 0.2882 1] Loop Sound
  (`/Engine/EditorBlueprintResources/StandardMacros.DoOnce` false :!label _label_3
    (:`Completed`
      (if (`self.LoopSound-Use?`)
        (bind _returnvalue (`GameplayStatics.SpawnSoundAtLocation` (`self.Loop Sound`) _current_location (struct) (`self.Loop Volume`) 1.0 0.0 (`self.Attenuation Settings`) null))
        (set `self.LoopSoundRef` _returnvalue)
        (`AudioComponent.FadeIn` _loopsoundref (`self.Loop Fade in Duration`) 1.0 0.0 "Linear")
        (if (`self.IsActivated?`) :!label _label_4
          (`SceneComponent.K2_SetWorldLocation` _loopsoundref _current_location false false)
          (`KismetSystemLibrary.Delay` 0.0)
          (goto _label_4)
          (else
            (`AudioComponent.FadeOut` _loopsoundref (`self.Alpha`) 0.0 "Linear")
            (goto _label_3 :!via `Reset`)))))))

(event `self.ReceiveTick`
  (params (DeltaSeconds :type "Float (single-precision)"))
  (bind _as_character (`self.As Character`))
  (bind _bp_scanspawn_actor_ref (`self.BP_ScanSpawn Actor Ref`))
  (bind _niagara (`/Game/ScanGridEffect/Blueprints/BP_ScanSpwan.Niagara` _bp_scanspawn_actor_ref))
  (bind _rootcomponent (`Actor.RootComponent` _as_character))
  (bind _returnvalue (`SceneComponent.K2_GetComponentLocation` _rootcomponent))
  (`self.UpdateScanTime` DeltaSeconds)
  (switch `/Game/ScanGridEffect/Materials/MaterialFunctions/ScanState` (`self.GetScanState`)
    (:`NewEnumerator0`
      ;[0.1892 0.4201 1] Activate Blend Weight only if PP_Scan is not destroyed
      (`self.UpdateScanPPBlendWeight` :!label _label_5)
      ;[0.2904 0.5242 1] Set BP_PP_Niagara System Asset, after "BP_ScanSpwan" spawned
      (if (`self.Use Niagara?`)
        (`NiagaraComponent.SetAsset` (`/Game/ScanGridEffect/Blueprints/BP_ScanSpwan.Niagara` (`self.BP_ScanSpawn Actor Ref`)) (`self.N_Scan`) false)))
    (:`NewEnumerator1`
      _)
    (:`NewEnumerator2`
      (goto _label_5))
    (:`NewEnumerator3`
      _))
  ;[0.7274 0.395 1] Update PP_Scan Location
  (`/Engine/EditorBlueprintResources/StandardMacros.IsValid` _as_character
    (:`Is Valid`
      (`/Engine/EditorBlueprintResources/StandardMacros.IsValid` _rootcomponent
        (:`Is Valid`
          (set `self.Current Location` _returnvalue)
          (`KismetMaterialLibrary.SetVectorParameterValue` "/Game/ScanGridEffect/Materials/MaterialFunctions/MPC_Scan.MPC_Scan" "Location" (`KismetMathLibrary.Conv_VectorToLinearColor` _returnvalue))
          ;[1 0.4842 0.8851] Niagara: Set Location & Parameters:
          (if (`self.Use Niagara?`)
            (`/Engine/EditorBlueprintResources/StandardMacros.IsValid` _bp_scanspawn_actor_ref
              (:`Is Valid`
                (`SceneComponent.K2_SetWorldLocation` _niagara (`KismetMathLibrary.Vector_SnappedToGrid` (`self.Current Location`) (`self.GridCellSize`)) false true)
                (`FXSystemComponent.SetColorParameter` _niagara "GridLines ColorX" (`self.LinesGrid Color X`))
                (`FXSystemComponent.SetColorParameter` _niagara "GridLines ColorY" (`self.LinesGrid Color Y`))
                (`FXSystemComponent.SetColorParameter` _niagara "GridLines ColorZ" (`self.LinesGrid Color Z`))
                (`FXSystemComponent.SetFloatParameter` _niagara "Lines Size" (`self.LinesGrid Size`))
                (`FXSystemComponent.SetColorParameter` _niagara "DotsGrid Color" (`self.DotsGrid Color`))
                (`FXSystemComponent.SetFloatParameter` _niagara "DotsGrid Size" (`self.DotsGrid Size`))))))))))

(event `self.ReceiveBeginPlay`
  (bind _pulsespeed (`self.PulseSpeed`))
  (set `self.IsActivated?` false)
  ;[0 1 0] Set your own Player Character Here
  (bind _ascharacter (cast `Character` (`self.GetOwner`))
    (:`then`
      (set `self.As Character` _ascharacter)
      (`self.UpdateScanState` "NewEnumerator2" true)
      ;[0.952 1 0.4733] Intialize PP_Scan Mat.Collection Parameters
      (`KismetMaterialLibrary.SetScalarParameterValue` "/Game/ScanGridEffect/Materials/MaterialFunctions/MPC_Scan.MPC_Scan" "GridCellSize" (`self.GridCellSize`))
      (`KismetMaterialLibrary.SetScalarParameterValue` "/Game/ScanGridEffect/Materials/MaterialFunctions/MPC_Scan.MPC_Scan" "Range" (`self.Range`))
      (`KismetMaterialLibrary.SetScalarParameterValue` "/Game/ScanGridEffect/Materials/MaterialFunctions/MPC_Scan.MPC_Scan" "PulseSpeed" _pulsespeed)
      ;[0.1765 0.5238 1] Initialize Sound timer
      (set `self.SoundTimeDelay` (/ 1.0 _pulsespeed)))
    (:`CastFailed`
      (`self.UpdateScanState` "NewEnumerator4" true))))

(event `StartSound`
  ;[0 0.2882 1] Start & End Sounds
  (if (`self.Start Sound-Use?`)
    (`/Engine/EditorBlueprintResources/StandardMacros.DoOnce` false :!label _label_6
      (:`Completed`
        (`GameplayStatics.SpawnSoundAtLocation` (`self.Start Sound`) (`self.Current Location`) (struct) (`self.Start Volume`) 1.0 0.0 (`self.Attenuation Settings`) null)
        ;;[0.000555 0 1] Pulse Sounds
        (`|ExecutionSequence`
          (:`then_0`
            (if (`self.IsActivated?`) :!label _label_7
              (`KismetSystemLibrary.Delay` 0.0)
              (goto _label_7)
              (else
                (goto _label_6 :!via `Reset`))))
          (:`then_1`
            (if (`self.PulseSound-Use?`)
              (`self.StartPulseSound`))))))))

(event `EndSound`
  ;[0 0.2882 1] Start & End Sounds
  (if (`self.End Sound-Use?`)
    (`/Engine/EditorBlueprintResources/StandardMacros.DoOnce` false :!label _label_8
      (:`Completed`
        (`GameplayStatics.SpawnSoundAtLocation` (`self.End Sound`) (`self.Current Location`) (struct) (`self.End Volume`) 1.0 0.0 (`self.Attenuation Settings`) null)
        (if (`self.IsActivated?`) :!label _label_9
          (goto _label_8 :!via `Reset`)
          (else
            (`KismetSystemLibrary.Delay` 0.0)
            (goto _label_9)))))))

(fn `EndScan`
  (returns (Ended :type Boolean))
  (switch `/Game/ScanGridEffect/Materials/MaterialFunctions/ScanState` (`self.GetScanState`)
    (:`NewEnumerator0`
      _)
    (:`NewEnumerator1`
      _)
    (:`NewEnumerator2`
      (return false))
    (:`NewEnumerator3`
      (return false))
    (:`NewEnumerator4`
      (return false)))
  ;[0.3125 1 0.8415] Reset Fade Out State
  (bind _updated (`self.UpdateScanState` "NewEnumerator2"))
  (return _updated))

(fn `GetScanPP Actor`
  (returns (NewParam :type "/Game/ScanGridEffect/Blueprints/BP_ScanSpwan Object Reference"))
  (bind _bp_scanspawn_actor_ref (`self.BP_ScanSpawn Actor Ref`))
  (bind _pp_material (`self.PP_Material`))
  (bind _postprocess (`/Game/ScanGridEffect/Blueprints/BP_ScanSpwan.PostProcess` (`self.BP_ScanSpawn Actor Ref`)))
  ;[1 0.2031 0.2031] Spawn PP Scan in the level at runtime
  (`/Engine/EditorBlueprintResources/StandardMacros.IsValid` _bp_scanspawn_actor_ref
    (:`Is Valid`
      (return _bp_scanspawn_actor_ref))
    (:`Is Not Valid`
      (bind _returnvalue (`|SpawnActorFromClass` "/Game/ScanGridEffect/Blueprints/BP_ScanSpwan.BP_ScanSpwan_C" (`KismetMathLibrary.MakeTransform` (0.0 0.0 0.0)) "Undefined" "OverrideRootScale" null null))
      (set `self.BP_ScanSpawn Actor Ref` _returnvalue)
      (`|ExecutionSequence`
        (:`then_0`
          (`/Engine/EditorBlueprintResources/StandardMacros.IsValid` (`self.PP_MaterialInstanceDynamic`)
            (:`Is Valid`
              _)
            (:`Is Not Valid`
              ;[0.3065 0.3381 1] If the PP_Material is not set, then create it here
              (`/Engine/EditorBlueprintResources/StandardMacros.IsValid` _pp_material
                (:`Is Valid`
                  (bind _returnvalue_2 (`KismetMaterialLibrary.CreateDynamicMaterialInstance` _pp_material))
                  (set `self.PP_MaterialInstanceDynamic` _returnvalue_2)))))
          (`/Engine/EditorBlueprintResources/StandardMacros.IsValid` _postprocess
            (:`Is Valid`
              (setmembers `PostProcessSettings` :`StructRef` (`PostProcessComponent.Settings` _postprocess) :`WeightedBlendables` (make `WeightedBlendables` (`|MakeArray` (make `WeightedBlendable` 1.0 (`self.PP_MaterialInstanceDynamic`))))))))
        (:`then_1`
          (return _bp_scanspawn_actor_ref))))))

(fn `GetScanState`
  (returns (NewParam :type "/Game/ScanGridEffect/Materials/MaterialFunctions/ScanState Enum"))
  (return (`self.State`)))

(fn `StartScan`
  (returns (Started :type Boolean))
  (switch `/Game/ScanGridEffect/Materials/MaterialFunctions/ScanState` (`self.GetScanState`)
    (:`NewEnumerator0`
      _)
    (:`NewEnumerator1`
      _)
    (:`NewEnumerator2`
      ;[0.3125 1 0.8415] Reset Fade In State
      (bind _updated (`self.UpdateScanState` "NewEnumerator0" :!label _label))
      (return _updated))
    (:`NewEnumerator3`
      (goto _label))
    (:`NewEnumerator4`
      _))
  (return false))

(fn `UpdateScanPPBlendWeight`
  (bind _scanfadingcurve (`self.ScanFadingCurve`))
  (bind _scannormalizedtime (`self.ScanNormalizedTime`))
  ;[1 0.2532 0.6284] Blend Weight Curve to smooth Fade In/Out
  (`/Engine/EditorBlueprintResources/StandardMacros.IsValid` _scanfadingcurve
    (:`Is Valid`
      (set `self.CurrentBlendWeight` (`CurveFloat.GetFloatValue` _scanfadingcurve _scannormalizedtime)))
    (:`Is Not Valid`
      (set `self.CurrentBlendWeight` _scannormalizedtime)))
  (bind _newparam (`self.GetScanPP Actor`))
  (`/Engine/EditorBlueprintResources/StandardMacros.IsValid` _newparam
    (:`Is Valid`
      (bind _postprocess (`/Game/ScanGridEffect/Blueprints/BP_ScanSpwan.PostProcess` _newparam))
      (`/Engine/EditorBlueprintResources/StandardMacros.IsValid` _postprocess
        (:`Is Valid`
          (set `PostProcessComponent.BlendWeight` (`self.CurrentBlendWeight`) _postprocess))))))

(fn `UpdateScanState`
  (params (State :type "/Game/ScanGridEffect/Materials/MaterialFunctions/ScanState Enum" :default "NewEnumerator0") (Force :type Boolean))
  (returns (Updated :type Boolean))
  (bind _bp_scanspawn_actor_ref (`self.BP_ScanSpawn Actor Ref`))
  (bind _bp_scanspawn_actor_ref_2 (`self.BP_ScanSpawn Actor Ref`))
  (if (or Force (`|EnumInequality` State (`self.State`)))
    (`|ExecutionSequence`
      (:`then_0`
        ;[1 1 1] Exit current state
        (switch `/Game/ScanGridEffect/Materials/MaterialFunctions/ScanState` (`self.State`)
          (:`NewEnumerator1`
            ;[0.3518 0.5139 1] Set PP_Scan material Fade In/Out final Statevalue
            (`KismetMaterialLibrary.SetScalarParameterValue` "/Game/ScanGridEffect/Materials/MaterialFunctions/MPC_Scan.MPC_Scan" "FadeIn"))
          (:`NewEnumerator3`
            (`KismetMaterialLibrary.SetScalarParameterValue` "/Game/ScanGridEffect/Materials/MaterialFunctions/MPC_Scan.MPC_Scan" "FadeOut")
            (`self.SetComponentTickEnabled` true)
            ;[1 0.1458 0.1458] Activate/Deactivate Niagara
            (if (`self.Use Niagara?`)
              (`/Engine/EditorBlueprintResources/StandardMacros.IsValid` _bp_scanspawn_actor_ref_2
                (:`Is Valid`
                  (`SceneComponent.SetVisibility` (`/Game/ScanGridEffect/Blueprints/BP_ScanSpwan.Niagara` _bp_scanspawn_actor_ref_2) true false)))))))
      (:`then_1`
        ;[1 1 1] Enter new state
        (bind _output_get (set `self.State` State))
        (switch `/Game/ScanGridEffect/Materials/MaterialFunctions/ScanState` _output_get
          (:`NewEnumerator1`
            (`KismetMaterialLibrary.SetScalarParameterValue` "/Game/ScanGridEffect/Materials/MaterialFunctions/MPC_Scan.MPC_Scan" "FadeIn" 1.0)
            (`self.UpdateScanPPBlendWeight`))
          (:`NewEnumerator3`
            (`KismetMaterialLibrary.SetScalarParameterValue` "/Game/ScanGridEffect/Materials/MaterialFunctions/MPC_Scan.MPC_Scan" "FadeOut" 1.0)
            (`|ExecutionSequence`
              (:`then_0`
                (if (`self.Use Niagara?`)
                  (`/Engine/EditorBlueprintResources/StandardMacros.IsValid` _bp_scanspawn_actor_ref
                    (:`Is Valid`
                      (`SceneComponent.SetVisibility` (`/Game/ScanGridEffect/Blueprints/BP_ScanSpwan.Niagara` _bp_scanspawn_actor_ref) false false)))))
              (:`then_1`
                (`self.UpdateScanPPBlendWeight`)
                (`self.SetComponentTickEnabled` false :!label _label)
                ;[1 0.9101 0.302] Destroy PP Scan in the level
                (`Actor.K2_DestroyActor` (`self.BP_ScanSpawn Actor Ref`))
                (set `self.BP_ScanSpawn Actor Ref` null))))
          (:`NewEnumerator4`
            (goto _label))))
      (:`then_2`
        (return true)))
    (else
      (return false))))

(fn `UpdateScanTime`
  (params (DeltaTime :type "Float (double-precision)"))
  (returns (Updated :type Boolean))
  (`|ExecutionSequence`
    (:`then_0`
      ;[1 0.4582 0.4682] Select Timer Direction:
      ; (0 to 1)
      ; (1 to 0)
      (switch `/Game/ScanGridEffect/Materials/MaterialFunctions/ScanState` (`self.GetScanState`)
        (:`NewEnumerator0`
          ;[0.2102 0.3584 1] Blend Timer value between 0 and 1
          (bind _output_get (set `self.ScanNormalizedTime` (+ (`self.ScanNormalizedTime`) (* (`local.DeltaTime`) (`self.FadeInSpeed`)))))
          (if (>= _output_get 1.0)
            ;[0.2102 0.3584 1] Set Timer final value
            (set `self.ScanNormalizedTime` 1.0)
            (`self.UpdateScanState` "NewEnumerator1")))
        (:`NewEnumerator2`
          (bind _output_get_2 (set `self.ScanNormalizedTime` (- (`self.ScanNormalizedTime`) (* (`local.DeltaTime`) (`self.FadeOutSpeed`)))))
          (if (<= _output_get_2 0.0)
            (set `self.ScanNormalizedTime` 0.0)
            (`self.UpdateScanState` "NewEnumerator3")))
        (:`NewEnumerator4`
          (return false)))
      (`KismetMaterialLibrary.SetScalarParameterValue` "/Game/ScanGridEffect/Materials/MaterialFunctions/MPC_Scan.MPC_Scan" "NormalizedTime" (`self.ScanNormalizedTime`)))
    (:`then_1`
      (return true))))