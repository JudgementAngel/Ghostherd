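; Base actor for procedural prop clusters that arranges the AA_StaticMeshComponent children of AARoot in the construction script.
; Place mode can hide a percentage of meshes using an optionally shuffled index list, then applies per-component random location, rotation and scale offsets to visible ones.
; A vertical line trace gates placement and supplies optional ground snapping and normal alignment.
; Scatter mode instead randomizes relative XY within ±ScatterRadius, optionally seeded.
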(event EventBeginPlay)

(event Collision|EventActorBeginOverlap
  (params (OtherActor :type Actor%20Object%20Reference)))

(event EventTick
  (params (DeltaSeconds :type Float%20%28single-precision%29)))

(fn ConstructionScript
  (bind _aa_root (Variables|Default|GetAA_Root))
  (bind _children (Components|GetChildrenComponents _aa_root false))
  (switch Utilities|FlowControl|Switch|SwitchonAggregatedActorMode (Variables|Default|GetAAMode)
    (:NewEnumerator2
      (if (Variables|Visible|GetUseVisible)
        (Utilities|FlowControl|Sequence
          (:then_0
            (if (Variables|Visible|GetVisibleRandom)
              (Utilities|Array|Clear (Variables|Visible|GetHideOrderIndex)))
            (for (_array_element _array_index) (Components|GetChildrenComponents (Variables|Default|GetAA_Root) false)
              (bind _asaa_static_mesh_component (Utilities|Casting|CastToAA_StaticMeshComponent _array_element))
              (Default|SetAASMCVisibility _asaa_static_mesh_component true)
              (if (Variables|Visible|GetVisibleRandom)
                (Utilities|Array|SetArrayElem (Variables|Visible|GetHideOrderIndex) _array_index _array_index true))))
          (:then_1
            (if (Variables|Visible|GetVisibleRandom)
              (Utilities|Array|Shuffle)))
          (:then_2
            (bind _index (Utilities|FlowControl|ForLoopwithBreak 0 (- (Math|Float|Truncate (* (Utilities|Array|Length _children) (- 1.0 (Variables|Visible|GetVisiblePercentage)))) 1))
              (:LoopBody
                (bind _asaa_static_mesh_component_2 (Utilities|Casting|CastToAA_StaticMeshComponent (Utilities|Array|Get(acopy) _children (Utilities|Array|Get(acopy) (Variables|Visible|GetHideOrderIndex) _index))))
                (Default|SetAASMCVisibility _asaa_static_mesh_component_2 false))))
          (:then_3
            (for _array_element_2 (Components|GetChildrenComponents (Variables|Default|GetAA_Root) false) :!label _label
              (bind _asaa_static_mesh_component_3 (Utilities|Casting|CastToAA_StaticMeshComponent _array_element_2))
              (if (Default|GetAASMCVisibility _asaa_static_mesh_component_3)
                (bind (_canplace _newtransform) (CallFunction|FindPlaceTransform _asaa_static_mesh_component_3))
                (if _canplace
                  (Transformation|SetWorldTransform _asaa_static_mesh_component_3 _newtransform false false))))))
        (else
          (goto _label))))
    (:NewEnumerator1
      (for _array_element_3 (Components|GetChildrenComponents (Variables|Default|GetAA_Root) false)
        (bind _asaa_static_mesh_component_4 (Utilities|Casting|CastToAA_StaticMeshComponent _array_element_3))
        (CallFunction|DealScatter _asaa_static_mesh_component_4)))))

(fn VectorAtoBRotateMatrix
  (params (VectorA :type Vector) (VectorB :type Vector))
  (LocalVariables|Setva VectorA)
  (LocalVariables|Setvb VectorB)
  (bind _output_get (LocalVariables|Setvs (Math|Vector|CrossProduct (LocalVariables|Getvb) (LocalVariables|Getva))))
  (LocalVariables|Setv (Math|Vector|Normalize _output_get))
  (bind _output_get_2 (LocalVariables|Setca (Math|Vector|DotProduct (LocalVariables|Getvb) (LocalVariables|Getva))))
  (LocalVariables|Setscale (- 1.0 _output_get_2))
  (LocalVariables|Setvt (* (LocalVariables|Getv) (LocalVariables|Getscale)))
  (LocalVariables|Setrm00 (+ (* (.x (LocalVariables|Getvt)) (.x (LocalVariables|Getv))) (LocalVariables|Getca)))
  (LocalVariables|Setrm11 (+ (* (.y (LocalVariables|Getvt)) (.y (LocalVariables|Getv))) (LocalVariables|Getca)))
  (LocalVariables|Setrm22 (+ (* (.z (LocalVariables|Getvt)) (.z (LocalVariables|Getv))) (LocalVariables|Getca)))
  (LocalVariables|Setvt (Math|Vector|MakeVector (* (.x (LocalVariables|Getvt)) (.y (LocalVariables|Getv))) (* (.y (LocalVariables|Getvt)) (.z (LocalVariables|Getv))) (* (.z (LocalVariables|Getvt)) (.x (LocalVariables|Getv)))))
  (LocalVariables|Setrm01 (- (.x (LocalVariables|Getvt)) (.z (LocalVariables|Getvs))))
  (LocalVariables|Setrm02 (- (.z (LocalVariables|Getvt)) (.y (LocalVariables|Getvs))))
  (LocalVariables|Setrm10 (- (.x (LocalVariables|Getvt)) (.z (LocalVariables|Getvs))))
  (LocalVariables|Setrm12 (- (.y (LocalVariables|Getvt)) (.x (LocalVariables|Getvs))))
  (LocalVariables|Setrm20 (- (.z (LocalVariables|Getvt)) (.y (LocalVariables|Getvs))))
  (LocalVariables|Setrm21 (- (.y (LocalVariables|Getvt)) (.x (LocalVariables|Getvs))))
  (return (Utilities|Struct|MakeMatrix (Utilities|Struct|MakePlane 0.0 (LocalVariables|Getrm00) (LocalVariables|Getrm01) (LocalVariables|Getrm02)) (Utilities|Struct|MakePlane 0.0 (LocalVariables|Getrm10) (LocalVariables|Getrm11) (LocalVariables|Getrm12)) (Utilities|Struct|MakePlane 0.0 (LocalVariables|Getrm20) (LocalVariables|Getrm21) (LocalVariables|Getrm22)) (Utilities|Struct|MakePlane 0.0 0.0 0.0 0.0))))

(fn FindPlaceTransform
  (params (AASMC :type AA%20Static%20Mesh%20Component%20Object%20Reference))
  (CallFunction|RandomLocation AASMC)
  (bind (_returnvalue _placelocation _placenormal) (CallFunction|CastRay AASMC 5e+03))
  (bind _newlocation (CallFunction|DealLocation _placelocation _placenormal AASMC))
  (bind _newrotation (CallFunction|DealRotation _placelocation _placenormal AASMC))
  (bind _newscale (CallFunction|DealScale "0, 0, 0" "0, 0, 0" AASMC))
  (return _returnvalue (Math|Transform|MakeTransform _newlocation _newrotation _newscale)))

(fn CastRay
  (params (AASMC :type AA%20Static%20Mesh%20Component%20Object%20Reference) (RayLength :type Float%20%28double-precision%29))
  (bind _returnvalue (Transformation|GetWorldTransform AASMC))
  (bind (_outhit _returnvalue_2) (Collision|LineTraceByChannel (+ (.location _returnvalue) (Math|Vector|MakeVector 0.0 0.0 RayLength)) (+ (.location _returnvalue) (Math|Vector|MakeVector 0.0 0.0 (* RayLength -1.0))) "TraceTypeQuery1" false 0 "None"))
  (return _returnvalue_2 (.Location (Collision|BreakHitResult _outhit)) (.Normal (Collision|BreakHitResult _outhit))))

(fn DealLocation
  (params (Location :type Vector) (Normal :type Vector) (AASMC :type AA%20Static%20Mesh%20Component%20Object%20Reference))
  (bind _relativelocation (Variables|/Script/Engine.SceneComponent|GetRelativeLocation AASMC))
  (return (Math|Vector|SelectVector (+ Location (Math|Vector|SelectVector (* (.z _relativelocation) Normal) (Math|Vector|MakeVector 0.0 0.0 (.z _relativelocation)) (Variables|/Game/Delete/PCG/BluePrints/AA_StaticMeshComponent.AA_StaticMeshComponent_C|GetIsGroundNormalZOffset AASMC))) (Transformation|GetWorldLocation AASMC) (Variables|/Game/Delete/PCG/BluePrints/AA_StaticMeshComponent.AA_StaticMeshComponent_C|GetSnapToGround AASMC))))

(fn DealRotation
  (params (Location :type Vector) (Normal :type Vector) (AASMC :type AA%20Static%20Mesh%20Component%20Object%20Reference))
  (bind (_x _y) (Math|Vector|BreakVector Normal))
  (bind _returnvalue (Math|Rotator|FindLookatRotation (Math|Vector|MakeVector 0.0 0.0 1.0) Normal))
  (bind _rotationoffsetmin (Variables|/Game/Delete/PCG/BluePrints/AA_StaticMeshComponent.AA_StaticMeshComponent_C|GetRotationOffsetMin AASMC))
  (bind _rotationoffsetmax (Variables|/Game/Delete/PCG/BluePrints/AA_StaticMeshComponent.AA_StaticMeshComponent_C|GetRotationOffsetMax AASMC))
  (bind _rotationoffsetmin_2 (Variables|/Game/Delete/PCG/BluePrints/AA_StaticMeshComponent.AA_StaticMeshComponent_C|GetRotationOffsetMin AASMC))
  (bind _rotationoffsetmax_2 (Variables|/Game/Delete/PCG/BluePrints/AA_StaticMeshComponent.AA_StaticMeshComponent_C|GetRotationOffsetMax AASMC))
  (bind _randomrotationoffset (Variables|/Game/Delete/PCG/BluePrints/AA_StaticMeshComponent.AA_StaticMeshComponent_C|GetRandomRotationOffset AASMC))
  (bind _userandomstream (Variables|/Game/Delete/PCG/BluePrints/AA_StaticMeshComponent.AA_StaticMeshComponent_C|GetUseRandomStream AASMC))
  (bind _randomstream (Variables|/Game/Delete/PCG/BluePrints/AA_StaticMeshComponent.AA_StaticMeshComponent_C|GetRandomStream AASMC))
  (bind _relativerotation (Variables|/Script/Engine.SceneComponent|GetRelativeRotation AASMC))
  (bind _returnvalue_2 (Math|Random|RandomFloatinRange (.x _rotationoffsetmin) (.x _rotationoffsetmax)))
  (bind _returnvalue_3 (Math|Random|RandomFloatinRange (.y _rotationoffsetmin) (.y _rotationoffsetmax)))
  (bind _returnvalue_4 (Math|Random|RandomFloatinRangefromStream (.z _rotationoffsetmin_2) (.z _rotationoffsetmax_2) _randomstream))
  (bind _returnvalue_5 (Math|Random|RandomFloatinRangefromStream (.x _rotationoffsetmin_2) (.x _rotationoffsetmax_2) _randomstream))
  (bind _returnvalue_6 (Math|Random|RandomFloatinRangefromStream (.y _rotationoffsetmin_2) (.y _rotationoffsetmax_2) _randomstream))
  (bind _returnvalue_7 (Math|Conversions|ToQuaternion(Rotator) _relativerotation))
  (bind _returnvalue_8 (Math|Vector|MakeVector _x _y 0.0))
  (bind _returnvalue_9 (Math|Conversions|ToQuaternion(Rotator) _returnvalue))
  (bind _returnvalue_10 (Math|Random|RandomFloatinRange (.z _rotationoffsetmin) (.z _rotationoffsetmax)))
  (bind _returnvalue_11 (Math|Vector|MakeVector _returnvalue_2 _returnvalue_3 _returnvalue_10))
  (bind _returnvalue_12 (Math|Vector|MakeVector _returnvalue_5 _returnvalue_6 _returnvalue_4))
  (bind _returnvalue_13 (Math|Vector|Normalize _returnvalue_8))
  (bind _returnvalue_14 (* _returnvalue_7 _returnvalue_9))
  (bind _returnvalue_15 (Math|Vector|DotProduct "1.000000,0.000000,0.000000" _returnvalue_13))
  (bind _returnvalue_16 (Math|Vector|SelectVector _returnvalue_12 _returnvalue_11 _userandomstream))
  (bind _returnvalue_17 (Math|Vector|SelectVector _returnvalue_16 "0, 0, 0" _randomrotationoffset))
  (bind _returnvalue_18 (Class|KismetMathLibrary|DegAcos _returnvalue_15))
  (bind _returnvalue_19 (Math|Float|Absolute(Float) _returnvalue_18))
  (return (Class|KismetMathLibrary|QuatRotator (* (Math|Conversions|ToQuaternion(Rotator) (Math|Rotator|SelectRotator (Math|Rotator|SelectRotator (Math|Rotator|SelectRotator (Class|KismetMathLibrary|QuatRotator _returnvalue_14) (Class|KismetMathLibrary|QuatRotator (* _returnvalue_14 (Math|Conversions|ToQuaternion(Rotator) (Math|Rotator|SelectRotator "0, 0, 0" (Math|Vector|RotatorfromAxisandAngle "0.000000,0.000000,1.000000" (Math|Float|SelectFloat _returnvalue_19 (* _returnvalue_19 -1.0) (> (.z (Math|Vector|CrossProduct _returnvalue_8 "1.000000,0.000000,0.000000")) 0.0))) (<= (Math|Vector|Distance(Vector) Normal "0.000000,0.000000,1.000000") 0.0001))))) (Variables|/Game/Delete/PCG/BluePrints/AA_StaticMeshComponent.AA_StaticMeshComponent_C|GetIsRotationWithNormal AASMC)) _relativerotation (Variables|/Game/Delete/PCG/BluePrints/AA_StaticMeshComponent.AA_StaticMeshComponent_C|GetSnapToGround AASMC)) _relativerotation (Variables|/Game/Delete/PCG/BluePrints/AA_StaticMeshComponent.AA_StaticMeshComponent_C|GetIsRotation AASMC))) (Math|Conversions|ToQuaternion(Rotator) (Math|Rotator|MakeRotator (.x _returnvalue_17) (.y _returnvalue_17) (.z _returnvalue_17)))))))

(fn DealScale
  (params (Location :type Vector) (Normal :type Vector) (AASMC :type AA%20Static%20Mesh%20Component%20Object%20Reference))
  (bind _scaleoffsetmin (Variables|/Game/Delete/PCG/BluePrints/AA_StaticMeshComponent.AA_StaticMeshComponent_C|GetScaleOffsetMin AASMC))
  (bind _scaleoffsetmax (Variables|/Game/Delete/PCG/BluePrints/AA_StaticMeshComponent.AA_StaticMeshComponent_C|GetScaleOffsetMax AASMC))
  (bind _userandomstream (Variables|/Game/Delete/PCG/BluePrints/AA_StaticMeshComponent.AA_StaticMeshComponent_C|GetUseRandomStream AASMC))
  (bind _randomstream (Variables|/Game/Delete/PCG/BluePrints/AA_StaticMeshComponent.AA_StaticMeshComponent_C|GetRandomStream AASMC))
  (bind _returnvalue (Math|Random|RandomFloatinRange (.x _scaleoffsetmin) (.x _scaleoffsetmax)))
  (bind _returnvalue_2 (Math|Random|RandomFloatinRange (.y _scaleoffsetmin) (.y _scaleoffsetmax)))
  (bind _returnvalue_3 (Math|Random|RandomFloatinRangefromStream (.z _scaleoffsetmin) (.z _scaleoffsetmax) _randomstream))
  (bind _returnvalue_4 (Math|Random|RandomFloatinRangefromStream (.x _scaleoffsetmin) (.x _scaleoffsetmax) _randomstream))
  (bind _returnvalue_5 (Math|Random|RandomFloatinRangefromStream (.y _scaleoffsetmin) (.y _scaleoffsetmax) _randomstream))
  (bind _returnvalue_6 (Math|Random|RandomFloatinRange (.z _scaleoffsetmin) (.z _scaleoffsetmax)))
  (bind _returnvalue_7 (Math|Vector|MakeVector _returnvalue _returnvalue_2 _returnvalue_6))
  (bind _returnvalue_8 (Math|Vector|MakeVector _returnvalue_4 _returnvalue_5 _returnvalue_3))
  (bind _returnvalue_9 (Math|Vector|SelectVector _returnvalue_8 _returnvalue_7 _userandomstream))
  (bind _x (Class|KismetMathLibrary|BreakVector3f _returnvalue_9))
  (return (+ (Variables|/Script/Engine.SceneComponent|GetRelativeScale3D AASMC) (Math|Vector|SelectVector (Math|Vector|SelectVector (Math|Vector|MakeVector _x _x _x) _returnvalue_9 (Variables|/Game/Delete/PCG/BluePrints/AA_StaticMeshComponent.AA_StaticMeshComponent_C|GetUniformScale AASMC)) "0, 0, 0" (Variables|/Game/Delete/PCG/BluePrints/AA_StaticMeshComponent.AA_StaticMeshComponent_C|GetRandomScaleOffset AASMC)))))

(fn DealScatter
  (params (AASMC :type Scene%20Component%20Object%20Reference))
  (bind _randomseed (Variables|Scatter|GetRandomSeed))
  (bind _scatterradius (Variables|Scatter|GetScatterRadius))
  (bind _relativelocation (Variables|/Script/Engine.SceneComponent|GetRelativeLocation AASMC))
  (bind _scatterradius_2 (Variables|Scatter|GetScatterRadius))
  (if (Variables|Scatter|GetResetRandomSeed)
    (Math|Random|SetRandomStreamSeed (Variables|Scatter|GetRandomSeed) (Math|Conversions|ToInteger(Byte) (Class|KismetMathLibrary|RandomInteger64inRange -2147483648 2147483647))))
  (Transformation|SetRelativeLocation AASMC (Math|Vector|SelectVector (Math|Vector|MakeVector (Math|Random|RandomFloatinRangefromStream (* _scatterradius_2 -1.0) _scatterradius_2 _randomseed) (Math|Random|RandomFloatinRangefromStream (* _scatterradius_2 -1.0) _scatterradius_2 _randomseed) (.z _relativelocation)) (Math|Vector|MakeVector (Math|Random|RandomFloatinRange (* _scatterradius -1.0) _scatterradius) (Math|Random|RandomFloatinRange (* _scatterradius -1.0) _scatterradius) (.z _relativelocation)) (Variables|Scatter|GetUseSeed)) false false))

(fn RandomLocation
  (params (AASMC :type AA%20Static%20Mesh%20Component%20Object%20Reference))
  (bind _locationoffsetmax (Variables|/Game/Delete/PCG/BluePrints/AA_StaticMeshComponent.AA_StaticMeshComponent_C|GetLocationOffsetMax AASMC))
  (bind _locationoffsetmin (Variables|/Game/Delete/PCG/BluePrints/AA_StaticMeshComponent.AA_StaticMeshComponent_C|GetLocationOffsetMin AASMC))
  (bind _locationoffsetmax_2 (Variables|/Game/Delete/PCG/BluePrints/AA_StaticMeshComponent.AA_StaticMeshComponent_C|GetLocationOffsetMax AASMC))
  (bind _randomstream (Variables|/Game/Delete/PCG/BluePrints/AA_StaticMeshComponent.AA_StaticMeshComponent_C|GetRandomStream AASMC))
  (bind _locationoffsetmin_2 (Variables|/Game/Delete/PCG/BluePrints/AA_StaticMeshComponent.AA_StaticMeshComponent_C|GetLocationOffsetMin AASMC))
  (Transformation|SetRelativeLocation AASMC (+ (Variables|/Script/Engine.SceneComponent|GetRelativeLocation AASMC) (Math|Vector|SelectVector (Math|Vector|SelectVector (Math|Vector|MakeVector (Math|Random|RandomFloatinRangefromStream (.x _locationoffsetmin) (.x _locationoffsetmax_2) _randomstream) (Math|Random|RandomFloatinRangefromStream (.y _locationoffsetmin) (.y _locationoffsetmax_2) _randomstream) (Math|Random|RandomFloatinRangefromStream (.z _locationoffsetmin) (.z _locationoffsetmax_2) _randomstream)) (Math|Vector|MakeVector (Math|Random|RandomFloatinRange (.x _locationoffsetmin_2) (.x _locationoffsetmax)) (Math|Random|RandomFloatinRange (.y _locationoffsetmin_2) (.y _locationoffsetmax)) (Math|Random|RandomFloatinRange (.z _locationoffsetmin_2) (.z _locationoffsetmax))) (Variables|/Game/Delete/PCG/BluePrints/AA_StaticMeshComponent.AA_StaticMeshComponent_C|GetUseRandomStream AASMC)) "0, 0, 0" (Variables|/Game/Delete/PCG/BluePrints/AA_StaticMeshComponent.AA_StaticMeshComponent_C|GetRandomLocationOffset AASMC))) false false)
  (return))