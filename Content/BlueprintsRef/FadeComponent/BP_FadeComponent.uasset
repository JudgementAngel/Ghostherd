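; Fade component that tracks a normalized fade value through fade in, faded in, fade out and faded out states.
; StartFade and EndFade request transitions, which UpdateFadeState applies while firing enter and exit events for the two faded states.
; Tick moves the value at separate in and out speeds, advances the state at each limit and fires an update event.
; Ticking switches off on entering Faded Out and back on when leaving it.
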(event `self.ReceiveTick`
  (params (DeltaSeconds :type "Float (single-precision)"))
  (`self.UpdateFadeTime` DeltaSeconds))

(fn `EndFade`
  (returns (bEnded :type Boolean))
  (`self.EndFadeEvent`)
  (switch `/Game/BlueprintsRef/FadeComponent/E_FadeState` (`self.GetFadeState`)
    (:`NewEnumerator0`
      _)
    (:`NewEnumerator1`
      (bind _bupdate (`self.UpdateFadeState` "NewEnumerator3" :!label _label))
      (return _bupdate))
    (:`NewEnumerator2`
      (goto _label))
    (:`NewEnumerator3`
      _)
    (:`NewEnumerator4`
      _))
  (return false))

(fn `GetFadeState`
  (returns (State :type "/Game/BlueprintsRef/FadeComponent/E_FadeState Enum"))
  (return (`self.FadeState`)))

(fn `StartFade`
  (returns (bStarted :type Boolean))
  (`self.StartFadeEvent`)
  (switch `/Game/BlueprintsRef/FadeComponent/E_FadeState` (`self.GetFadeState`)
    (:`NewEnumerator0`
      _)
    (:`NewEnumerator1`
      (return false))
    (:`NewEnumerator2`
      (return false))
    (:`NewEnumerator3`
      _)
    (:`NewEnumerator4`
      _))
  (bind _bupdate (`self.UpdateFadeState` "NewEnumerator1"))
  (return _bupdate))

(fn `UpdateFadeState`
  (params (NewState :type "/Game/BlueprintsRef/FadeComponent/E_FadeState Enum" :default "NewEnumerator0") (bForce :type Boolean))
  (returns (bUpdate :type Boolean))
  (if (or bForce (`|EnumInequality` NewState (`self.FadeState`)))
    (`|ExecutionSequence`
      (:`then_0`
        (switch `/Game/BlueprintsRef/FadeComponent/E_FadeState` (`self.FadeState`) ; Exit Current State
          (:`NewEnumerator2`
            (`self.FadedInExitEvent`))
          (:`NewEnumerator4`
            (`self.FadedOutExitEvent`)
            (`self.SetComponentTickEnabled` true))))
      (:`then_1`
        (bind _output_get (set `self.FadeState` NewState))
        (switch `/Game/BlueprintsRef/FadeComponent/E_FadeState` _output_get ; Enter New State
          (:`NewEnumerator0`
            (`self.SetComponentTickEnabled` false :!label _label))
          (:`NewEnumerator2`
            (`self.FadedInEnterEvent`))
          (:`NewEnumerator4`
            (`self.FadedOutEnterEvent`)
            (goto _label)))))
    (else
      (return false))))

(fn `UpdateFadeTime`
  (params (DeltaTime :type "Float (double-precision)"))
  (returns (bUpdated :type Boolean))
  (`|ExecutionSequence`
    (:`then_0`
      (switch `/Game/BlueprintsRef/FadeComponent/E_FadeState` (`self.FadeState`)
        (:`NewEnumerator0`
          (return false))
        (:`NewEnumerator1`
          (bind _output_get (set `self.FadeNormalizeTime` (+ (`self.FadeNormalizeTime`) (* (`local.DeltaTime`) (`self.FadeInSpeed`)))))
          (if (>= _output_get 1.0)
            (set `self.FadeNormalizeTime` 1.0)
            (`self.UpdateFadeState` "NewEnumerator2")))
        (:`NewEnumerator3`
          (bind _output_get_2 (set `self.FadeNormalizeTime` (- (`self.FadeNormalizeTime`) (* (`local.DeltaTime`) (`self.FadeOutSpeed`)))))
          (if (<= _output_get_2 0.0)
            (set `self.FadeNormalizeTime` 0.0)
            (`self.UpdateFadeState` "NewEnumerator4")))))
    (:`then_1`
      (`self.FadeUpdateEvent`))
    (:`then_2`
      (return true))))